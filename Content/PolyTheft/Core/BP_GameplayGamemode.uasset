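; Gameplay game mode that randomly places the keys for the level's locks when play begins.
; PrepareKeys gathers all BP_Lock and BP_KeySpawnPoint actors, then shuffles the spawn points.
; Each lock is paired by index with a point, which spawns a key carrying that lock's required key code.
; An on-screen error prints when there are fewer points than locks.
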(event `self.ReceiveBeginPlay`
  (`self.PrepareKeys`))

(fn `PrepareKeys`
  (locals (Locks :type "Array of /Game/PolyTheft/Actors/Puzzles/KeyPuzzle/BP_Lock Object Reference") (Points :type "Array of /Game/PolyTheft/Actors/Puzzles/KeyPuzzle/BP_KeySpawnPoint Object Reference"))
  (bind _outactors (`GameplayStatics.GetAllActorsOfClass` "/Game/PolyTheft/Actors/Puzzles/KeyPuzzle/BP_Lock.BP_Lock_C"))
  (set `local.Locks` _outactors)
  (bind _outactors_2 (`GameplayStatics.GetAllActorsOfClass` "/Game/PolyTheft/Actors/Puzzles/KeyPuzzle/BP_KeySpawnPoint.BP_KeySpawnPoint_C"))
  (set `local.Points` _outactors_2)
  (`KismetArrayLibrary.Array_Shuffle` (`local.Points`))
  (for (_array_element _array_index) (`local.Locks`)
    (if (> (`KismetArrayLibrary.Array_Length` (`local.Points`)) _array_index)
      (`/Game/PolyTheft/Actors/Puzzles/KeyPuzzle/BP_KeySpawnPoint.SpawnKey` (`|GetArrayItem` (`local.Points`) _array_index) (`/Game/PolyTheft/Actors/Puzzles/KeyPuzzle/BP_Lock.KeyCodeRequied` _array_element))
      (else
        (`KismetSystemLibrary.PrintString` "ERROR: Cant spawn, not enought points." true true (struct :`R` 0.640625 :`B` 0.027946 :`A` 1.0) 30.0)))))

(fn `UserConstructionScript`)