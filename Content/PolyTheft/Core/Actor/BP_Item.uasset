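; BP_Item is a pickup actor that puts an item into the inventory when interacted with.
; Its item data comes from the DT_ItemInfo data table row named by RowName.
; Interaction enter and exit events show and hide the HUD's PickupInfo prompt with that data.
; On interact it passes the data to the inventory component, then hides the prompt and destroys itself only if the add succeeds.
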(event `/Game/PolyTheft/Core/Interfaces/BPI_Interaction.OnInteract`
  (bind _success (`/Game/PolyTheft/Core/Components/BP_InventoryComponent.AddItem` (`/Game/PolyTheft/Core/BlueprintLibrary/BPFL_Getters.GetInventoryComponent`) (`self.GetData`)))
  (if _success
    (`/Game/PolyTheft/UI/WBP_PickupInfo.HidePrompt` (`/Game/PolyTheft/UI/WBP_HeadsUpDisplay.PickupInfo` (`/Game/PolyTheft/Core/BlueprintLibrary/BPFL_Getters.GetGameHud`)))
    (`self.K2_DestroyActor`)))

(event `/Game/PolyTheft/Core/Interfaces/BPI_Interaction.OnInteractionEnter`
  (`/Game/PolyTheft/UI/WBP_PickupInfo.ShowPrompt` (`/Game/PolyTheft/UI/WBP_HeadsUpDisplay.PickupInfo` (`/Game/PolyTheft/Core/BlueprintLibrary/BPFL_Getters.GetGameHud`)) (`self.GetData`)))

(event `/Game/PolyTheft/Core/Interfaces/BPI_Interaction.OnInteractionExit`
  (`/Game/PolyTheft/UI/WBP_PickupInfo.HidePrompt` (`/Game/PolyTheft/UI/WBP_HeadsUpDisplay.PickupInfo` (`/Game/PolyTheft/Core/BlueprintLibrary/BPFL_Getters.GetGameHud`))))

(fn `GetData`
  (returns (`Out Row` :type "ItemInfo Structure"))
  (bind _returnvalue (`|GetDataTableRow` "/Game/PolyTheft/DataTable/DT_ItemInfo.DT_ItemInfo" (`self.Row Name`))
    (:`then`
      (return _returnvalue))))

(fn `UserConstructionScript`)