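; BP_Lock is an interactable lock actor that opens only for a player carrying the key matching its required key code.
; Entering interaction range shows a HUD pickup prompt labeled with that code, and exiting hides it.
; On interact it queries the inventory component, then either hides the prompt and destroys itself or replaces the prompt with a missing-key message.
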(event `/Game/PolyTheft/Core/Interfaces/BPI_Interaction.OnInteract`
  (bind _pickupinfo (`/Game/PolyTheft/UI/WBP_HeadsUpDisplay.PickupInfo` (`/Game/PolyTheft/Core/BlueprintLibrary/BPFL_Getters.GetGameHud`)))
  (if (`/Game/PolyTheft/Core/Components/BP_InventoryComponent.HasKey` (`/Game/PolyTheft/Core/BlueprintLibrary/BPFL_Getters.GetInventoryComponent`) (`self.KeyCodeRequied`))
    (`/Game/PolyTheft/UI/WBP_PickupInfo.HidePrompt` _pickupinfo)
    (`self.K2_DestroyActor`)
    (else
      (`/Game/PolyTheft/UI/WBP_PickupInfo.HidePrompt` (`/Game/PolyTheft/UI/WBP_HeadsUpDisplay.PickupInfo` (`/Game/PolyTheft/Core/BlueprintLibrary/BPFL_Getters.GetGameHud`)))
      (`/Game/PolyTheft/UI/WBP_PickupInfo.ShowPrompt` _pickupinfo (make `ItemInfo` "Player has no requied key")))))

(event `/Game/PolyTheft/Core/Interfaces/BPI_Interaction.OnInteractionEnter`
  (`/Game/PolyTheft/UI/WBP_PickupInfo.ShowPrompt` (`/Game/PolyTheft/UI/WBP_HeadsUpDisplay.PickupInfo` (`/Game/PolyTheft/Core/BlueprintLibrary/BPFL_Getters.GetGameHud`)) (make `ItemInfo` (`KismetTextLibrary.Conv_StringToText` (`KismetStringLibrary.Concat_StrStr` "Lock - " (`self.KeyCodeRequied`))))))

(event `/Game/PolyTheft/Core/Interfaces/BPI_Interaction.OnInteractionExit`
  (`/Game/PolyTheft/UI/WBP_PickupInfo.HidePrompt` (`/Game/PolyTheft/UI/WBP_HeadsUpDisplay.PickupInfo` (`/Game/PolyTheft/Core/BlueprintLibrary/BPFL_Getters.GetGameHud`))))

(fn `UserConstructionScript`)