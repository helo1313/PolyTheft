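; BP_SlideingDoor is an interactable sliding door that toggles open and closed.
; Interaction enter and exit events show or hide a HUD prompt with the object name.
; Interacting flip-flops a timeline forward or in reverse, lerping the mesh's relative location between closed and open positions without sweep.
; The construction script applies an optional override mesh and, only when one is valid, can preview the open position through DebugOpen.
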(event `/Game/PolyTheft/Core/Interfaces/BPI_Interaction.OnInteractionExit`
  (`/Game/PolyTheft/UI/WBP_InteractionInfo.HidePrompt` (`/Game/PolyTheft/UI/WBP_HeadsUpDisplay.WBP_InteractionInfo` (`/Game/PolyTheft/Core/BlueprintLibrary/BPFL_Getters.GetGameHud`))))

(event `/Game/PolyTheft/Core/Interfaces/BPI_Interaction.OnInteractionEnter`
  (`/Game/PolyTheft/UI/WBP_InteractionInfo.ShowPrompt` (`/Game/PolyTheft/UI/WBP_HeadsUpDisplay.WBP_InteractionInfo` (`/Game/PolyTheft/Core/BlueprintLibrary/BPFL_Getters.GetGameHud`)) (`self.ObjectName`)))

(event `/Game/PolyTheft/Core/Interfaces/BPI_Interaction.OnInteract`
  (`/Engine/EditorBlueprintResources/StandardMacros.FlipFlop`
    (:`A`
      (bind (_direction _newtrack_0) (`Timeline|Timeline` :!label _label)
        (:`Update`
          (`SceneComponent.K2_SetRelativeLocation` (`self.StaticMesh`) (`KismetMathLibrary.VLerp` (`self.CloseLocation`) (`self.OpenLocation`) _newtrack_0) false false))))
    (:`B`
      (goto _label :!via `Reverse`))))

(fn `UserConstructionScript`
  (`/Engine/EditorBlueprintResources/StandardMacros.IsValid` (`self.OverrideMesh`)
    (:`Is Valid`
      (`StaticMeshComponent.SetStaticMesh` (`self.StaticMesh`) (`self.OverrideMesh`))
      (if (`self.DebugOpen`)
        (`SceneComponent.K2_SetRelativeLocation` (`self.StaticMesh`) (`self.OpenLocation`) false false)))))