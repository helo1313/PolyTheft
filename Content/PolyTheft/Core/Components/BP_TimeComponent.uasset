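; BP_TimeComponent is a component that runs an in-game clock, tracking minutes and hours.
; On BeginPlay it starts a looping timer that calls MinutePass at the interval set by RealTimeForMinutePass.
; MinutePass rolls overflowing minutes into HourPass, which wraps hours over a 24-hour cycle without tracking days.
; Each step calls OnMinutePass or OnHourPass before the wrap reset is applied.
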(event `self.ReceiveBeginPlay`
  (`KismetSystemLibrary.K2_SetTimer` null "MinutePass" (`self.RealTimeForMinutePass`) true))

(fn `HourPass`
  (bind _result (`/Engine/EditorBlueprintResources/StandardMacros.IncrementInt` (`self.Hour`))
    (:`  `
      (`self.OnHourPass`)
      (if (> _result 23)
        (set `self.Hour` 0)))))

(fn `MinutePass`
  (bind _result (`/Engine/EditorBlueprintResources/StandardMacros.IncrementInt` (`self.Minute`))
    (:`  `
      (`self.OnMinutePass`)
      (if (> _result 59)
        (set `self.Minute` 0)
        (`self.HourPass`)))))