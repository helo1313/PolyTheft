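; BP_InventoryComponent is an inventory component that stores items for PolyTheft and tracks their combined value and weight.
; AddItem appends an item and updates both running totals only when CanAddItem passes, returning whether it succeeded.
; CanAddItem checks that the new total weight stays within the weight limit and that the individual item's size does not exceed the size limit.
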(fn `AddItem`
  (params (Item :type "ItemInfo Structure"))
  (returns (Success :type Boolean))
  (bind (_name _weight _size _value) (break `ItemInfo` Item))
  (if (`self.CanAddItem` Item)
    (`KismetArrayLibrary.Array_Add` (`self.Items`) Item)
    (set `self.CurrentValue` (+ (`self.CurrentValue`) _value))
    (set `self.CurrentWeight` (+ (`self.CurrentWeight`) _weight))
    (return true)
    (else
      (return false))))

(fn `CanAddItem`
  (params (Item :type "ItemInfo Structure"))
  (returns (CanAdd :type Boolean))
  (bind (_name _weight _size) (break `ItemInfo` Item))
  (return (and (<= (+ (`self.CurrentWeight`) _weight) (`self.MaxWeight`)) (<= _size (`self.MaxSize`)))))