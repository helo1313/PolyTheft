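; Actor component for BP_Character that lets the player hover over and interact with actors implementing BPI_Interaction.
; Each tick it line-traces forward from the first-person camera, with debug drawing set to ForDuration.
; ProcessHit caches the hovered actor, sending enter and exit messages only when the target changes or is lost.
; RequestInteraction sends the interact message to the currently hovered actor, if valid.
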(event `self.ReceiveBeginPlay`
  (bind _asbp_character (cast `/Game/PolyTheft/Core/BP_Character` (`self.GetOwner`)))
  (set `self.As BP Character` _asbp_character))

(event `self.ReceiveTick`
  (params (DeltaSeconds :type "Float (single-precision)"))
  (bind _firstpersoncameracomponent (`PolyTheftCharacter.FirstPersonCameraComponent` (`self.As BP Character`)))
  (bind _returnvalue (`SceneComponent.K2_GetComponentLocation` _firstpersoncameracomponent))
  (bind _outhit (`KismetSystemLibrary.LineTraceSingle` :`Start` _returnvalue :`End` (+ _returnvalue (* (`SceneComponent.GetForwardVector` _firstpersoncameracomponent) (`self.TraceLenght`))) :`TraceChannel` "TraceTypeQuery3" :`DrawDebugType` "ForDuration"))
  (`self.ProcessHit` _outhit))

(event `RequestInteraction`
  (if (`KismetSystemLibrary.IsValid` (`self.CurrentHoverActor`))
    (message `/Game/PolyTheft/Core/Interfaces/BPI_Interaction.OnInteract` (`self.CurrentHoverActor`))))

(fn `ProcessHit`
  (params (HitResult :type "HitResult Structure"))
  (bind (_bblockinghit _binitialoverlap _time _distance _location _impactpoint _normal _impactnormal _physmat _hitactor) (`GameplayStatics.BreakHitResult` HitResult))
  (bind _currenthoveractor (`self.CurrentHoverActor`))
  (bind _currenthoveractor_2 (`self.CurrentHoverActor`))
  (if _bblockinghit
    (if (`KismetSystemLibrary.IsValid` _hitactor)
      (if (`KismetSystemLibrary.DoesImplementInterface` _hitactor "/Game/PolyTheft/Core/Interfaces/BPI_Interaction.BPI_Interaction_C")
        (if (!= (`self.CurrentHoverActor`) _hitactor)
          (if (`KismetSystemLibrary.IsValid` _currenthoveractor)
            (message `/Game/PolyTheft/Core/Interfaces/BPI_Interaction.OnInteractionExit` _currenthoveractor))
          (bind _output_get (set `self.CurrentHoverActor` _hitactor))
          (message `/Game/PolyTheft/Core/Interfaces/BPI_Interaction.OnInteractionEnter` _output_get))
        (else
          (if (`KismetSystemLibrary.IsValid` _currenthoveractor_2) :!label _label
            (message `/Game/PolyTheft/Core/Interfaces/BPI_Interaction.OnInteractionExit` _currenthoveractor_2))
          (set `self.CurrentHoverActor` null)))
      (else
        (goto _label)))
    (else
      (goto _label))))