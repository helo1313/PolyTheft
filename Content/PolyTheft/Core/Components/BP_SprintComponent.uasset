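; Actor component that gives BP_Character sprinting limited by a stamina pool.
; On BeginPlay it caches the owner's CharacterMovement and applies walk speed.
; StartSprint switches to sprint speed only above a minimum stamina, and StopSprint restores walk speed.
; Tick drains stamina while sprinting, stopping the sprint at zero, and otherwise regenerates it up to the maximum.
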(event `self.ReceiveBeginPlay`
  (bind _asbp_character (cast `/Game/PolyTheft/Core/BP_Character` (`self.GetOwner`)))
  (bind _output_get (set `self.Character Movement` (`Character.CharacterMovement` _asbp_character)))
  (set `CharacterMovementComponent.MaxWalkSpeed` (`self.WalkSpeed`) _output_get))

(event `StartSprint`
  (if (> (`self.Stamina`) (`self.MinimumStaminaForUse`))
    (set `self.bIsSprinting` true)
    (set `CharacterMovementComponent.MaxWalkSpeed` (`self.SprintSpeed`) (`self.Character Movement`))))

(event `StopSprint`
  (set `self.bIsSprinting` false)
  (set `CharacterMovementComponent.MaxWalkSpeed` (`self.WalkSpeed`) (`self.Character Movement`)))

(event `self.ReceiveTick`
  (params (DeltaSeconds :type "Float (single-precision)"))
  (if (`self.bIsSprinting`)
    (set `self.Stamina` (`KismetMathLibrary.FClamp` (- (`self.Stamina`) (* (`self.StaminaConsumeRate`) DeltaSeconds)) 0.0 (`self.MaxStamina`)))
    (if (<= (`self.Stamina`) 0.0)
      (`self.StopSprint`))
    (else
      (set `self.Stamina` (`KismetMathLibrary.FClamp` (+ (`self.Stamina`) (* DeltaSeconds (`self.StaminaRecoveryRate`))) 0.0 (`self.MaxStamina`))))))