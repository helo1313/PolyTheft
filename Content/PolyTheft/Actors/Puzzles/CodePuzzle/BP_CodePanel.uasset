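; BP_CodePanel is an interactable puzzle actor that presents a code-entry puzzle to the player.
; On interaction, while unsolved, it creates WBP_CodePuzzle, binds its success event, pauses the game and shows the mouse cursor.
; On success it removes the widget, restores play, marks itself solved and fires OnSolved for other objects to react to.
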(event `/Game/PolyTheft/Core/Interfaces/BPI_Interaction.OnInteract`
  (`parent.OnInteract`)
  (if (not (`self.bIsSolved`))
    (bind _returnvalue (`|CreateWidget` "/Game/PolyTheft/UI/Puzzles/CodePuzzle/WBP_CodePuzzle.WBP_CodePuzzle_C"))
    (add `/Game/PolyTheft/UI/Puzzles/CodePuzzle/WBP_CodePuzzle.OnSucces` _returnvalue (delegate `OnSuccess`))
    (`UserWidget.AddToViewport` _returnvalue 0)
    (`GameplayStatics.SetGamePaused` true)
    (set `PlayerController.bShowMouseCursor` true (`GameplayStatics.GetPlayerController` 0))))

(event `OnSuccess`
  (`KismetSystemLibrary.PrintString` "PUZZLE SOLVED" true true (struct :`R` 0.099913 :`G` 0.307292 :`A` 1.0))
  (`Widget.RemoveFromParent` (stale `/Game/PolyTheft/Core/Interfaces/BPI_Interaction.OnInteract` _returnvalue))
  (`GameplayStatics.SetGamePaused` false)
  (set `PlayerController.bShowMouseCursor` false (`GameplayStatics.GetPlayerController` 0))
  (set `self.bIsSolved` true)
  (`self.OnSolved`))

(fn `UserConstructionScript`)