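; BP_Key is a pickup key actor for the key puzzle, identified by its KeyCode.
; Entering interaction range shows a "Key" prompt with the code on the HUD's StaticItemInfo widget, and leaving hides it.
; Interacting adds the KeyCode to the inventory component, hides the prompt and destroys the actor.
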(event `/Game/PolyTheft/Core/Interfaces/BPI_Interaction.OnInteract`
  (`/Game/PolyTheft/Core/Components/BP_InventoryComponent.AddKey` (`/Game/PolyTheft/Core/BlueprintLibrary/BPFL_Getters.GetInventoryComponent`) (`self.KeyCode`))
  (`/Game/PolyTheft/UI/WBP_StaticItemInfo.HidePrompt` (`/Game/PolyTheft/UI/WBP_HeadsUpDisplay.StaticItemInfo` (`/Game/PolyTheft/Core/BlueprintLibrary/BPFL_Getters.GetGameHud`)))
  (`self.K2_DestroyActor`))

(event `/Game/PolyTheft/Core/Interfaces/BPI_Interaction.OnInteractionEnter`
  (`/Game/PolyTheft/UI/WBP_StaticItemInfo.ShowPrompt` (`/Game/PolyTheft/UI/WBP_HeadsUpDisplay.StaticItemInfo` (`/Game/PolyTheft/Core/BlueprintLibrary/BPFL_Getters.GetGameHud`)) "Key" (`KismetTextLibrary.Conv_StringToText` (`self.KeyCode`))))

(event `/Game/PolyTheft/Core/Interfaces/BPI_Interaction.OnInteractionExit`
  (`/Game/PolyTheft/UI/WBP_StaticItemInfo.HidePrompt` (`/Game/PolyTheft/UI/WBP_HeadsUpDisplay.StaticItemInfo` (`/Game/PolyTheft/Core/BlueprintLibrary/BPFL_Getters.GetGameHud`))))

(fn `UserConstructionScript`)