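; BP_Lock is an interactable lock actor for a key puzzle that opens when the player carries a key with the matching code.
; On interact it checks the inventory component for the required key code, then either calls its unlock notification and destroys itself or shows a missing-key prompt.
; Entering and leaving interaction range shows and hides a HUD prompt displaying the lock's code.
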(event `/Game/PolyTheft/Core/Interfaces/BPI_Interaction.OnInteract`
  (bind _staticiteminfo (`/Game/PolyTheft/UI/WBP_HeadsUpDisplay.StaticItemInfo` (`/Game/PolyTheft/Core/BlueprintLibrary/BPFL_Getters.GetGameHud`)))
  (if (`/Game/PolyTheft/Core/Components/BP_InventoryComponent.HasKey` (`/Game/PolyTheft/Core/BlueprintLibrary/BPFL_Getters.GetInventoryComponent`) (`self.KeyCodeRequied`))
    (`/Game/PolyTheft/UI/WBP_StaticItemInfo.HidePrompt` _staticiteminfo)
    (`self.OnUnlock`)
    (`self.K2_DestroyActor`)
    (else
      (`/Game/PolyTheft/UI/WBP_StaticItemInfo.HidePrompt` _staticiteminfo)
      (`/Game/PolyTheft/UI/WBP_StaticItemInfo.ShowPrompt` _staticiteminfo "No key with this code in inventory" (`KismetTextLibrary.Conv_StringToText` (`self.KeyCodeRequied`))))))

(event `/Game/PolyTheft/Core/Interfaces/BPI_Interaction.OnInteractionEnter`
  (`/Game/PolyTheft/UI/WBP_StaticItemInfo.ShowPrompt` (`/Game/PolyTheft/UI/WBP_HeadsUpDisplay.StaticItemInfo` (`/Game/PolyTheft/Core/BlueprintLibrary/BPFL_Getters.GetGameHud`)) "Lock" (`KismetTextLibrary.Conv_StringToText` (`self.KeyCodeRequied`))))

(event `/Game/PolyTheft/Core/Interfaces/BPI_Interaction.OnInteractionExit`
  (`/Game/PolyTheft/UI/WBP_StaticItemInfo.HidePrompt` (`/Game/PolyTheft/UI/WBP_HeadsUpDisplay.StaticItemInfo` (`/Game/PolyTheft/Core/BlueprintLibrary/BPFL_Getters.GetGameHud`))))

(fn `UserConstructionScript`)